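; BP_Ball is a bouncing ball actor that moves itself at a variable speed along a direction.
; Each tick, if its Ball reference is valid, it does a swept world offset and, on a blocking hit, reflects the direction about the surface normal.
; Each Hit event cuts the speed by a tenth, never below a minimum, and prints the result.
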(event EventBeginPlay)

(event Collision|EventActorBeginOverlap
  (params (OtherActor :type Actor%20Object%20Reference)))

(event EventTick
  (params (DeltaSeconds :type Float%20%28single-precision%29))
  (Utilities|IsValid (Variables|Default|GetBall)
    (:Is%20Valid
      (bind _sweephitresult (Transformation|AddActorWorldOffset (* (* (Variables|BallSetings|GetSpeed) (Variables|Default|GetDirection)) DeltaSeconds) true))
      (if (.bBlockingHit (Collision|BreakHitResult _sweephitresult))
        (Variables|Default|SetDirection (Math|Vector|GetReflectionVector (Variables|Default|GetDirection) (.Normal (Collision|BreakHitResult _sweephitresult))))))))

(event Collision|EventHit
  (params (MyComp :type Primitive%20Component%20Object%20Reference) (Other :type Actor%20Object%20Reference) (OtherComp :type Primitive%20Component%20Object%20Reference) (bSelfMoved :type Boolean) (HitLocation :type Vector :default "0, 0, 0") (HitNormal :type Vector :default "0, 0, 0") (NormalImpulse :type Vector :default "0, 0, 0") (Hit :type Hit%20Result%20Structure%20%28by%20ref%29))
  (bind _output_get (Variables|BallSetings|SetSpeed (Math|Float|Max(Float) (Variables|BallSetings|GetMinSpeed) (- (Variables|BallSetings|GetSpeed) (Math|Float|SafeDivide (Variables|BallSetings|GetSpeed) 1e+01)))))
  (Development|PrintString (Utilities|String|ToString(Float) _output_get)))

(fn ConstructionScript)